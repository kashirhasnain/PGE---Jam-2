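; BP_Car is a short-lived car hazard that kills the player character on overlap and destroys itself seven seconds after spawning.
; On BeginPlay it also creates a 2D sound and sets a body material through a three-color switch whose constant input always selects Color1.
; When its Box overlaps a ThirdPersonCharacter, it creates a glass-break sound, teleports the character to SpawnLocation and sets its Dead flag.
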(event `self.ReceiveBeginPlay`
  (bind _car (`self.Car`))
  (`|ExecutionSequence`
    (:`then_0`
      (`KismetSystemLibrary.Delay` 7.0)
      (`self.K2_DestroyActor`))
    (:`then_1`
      (switch `int` 0
        (:`0`
          (`PrimitiveComponent.SetMaterial` _car 3 "/Game/color1.color1"))
        (:`1`
          (`PrimitiveComponent.SetMaterial` _car 3 "/Game/color2.color2"))
        (:`2`
          (`PrimitiveComponent.SetMaterial` _car 3 "/Game/color3.color3"))))
    (:`then_2`
      (`GameplayStatics.CreateSound2D` "/Game/arabapitch.arabapitch" 5.0 1.0 0.0 null))))

(event `self.Box.OnComponentBeginOverlap`
  (params (OverlappedComponent :type "PrimitiveComponent Object Reference") (OtherActor :type "Actor Object Reference") (OtherComp :type "PrimitiveComponent Object Reference") (OtherBodyIndex :type Integer) (bFromSweep :type Boolean) (SweepResult :type "HitResult Structure (by ref)"))
  (bind _asthird_person_character (cast `/Game/ThirdPersonBP/Blueprints/ThirdPersonCharacter` OtherActor))
  (`GameplayStatics.CreateSound2D` "/Game/glass_break.glass_break" 1.0 1.0 0.0 null)
  (`SceneComponent.K2_SetWorldLocation` (`Actor.RootComponent` _asthird_person_character) (`self.Spawn_Location`) false true)
  (set `/Game/ThirdPersonBP/Blueprints/ThirdPersonCharacter.dead?` true _asthird_person_character))

(fn `UserConstructionScript`)