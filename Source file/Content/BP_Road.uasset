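; BP_Road is a road actor that randomly spawns BP_Car traffic from either of two directions.
; A Delay on Tick acts as a random repeating timer, followed by coin flips for spawning and direction.
; Cars spawn far offset from two arrows, with a Spawned-flag cooldown on one direction only.
; Spawning swaps the road material as an apparent warning, reverted when a car exits the Box.
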(event `self.ReceiveTick`
  (params (DeltaSeconds :type "Float (single-precision)"))
  (bind _arrow (`self.Arrow`))
  (bind _arrow2 (`self.Arrow2`))
  (`KismetSystemLibrary.Delay` (`KismetMathLibrary.RandomFloatInRange` 0.5 10.0))
  (switch `int` (`KismetMathLibrary.RandomIntegerInRange` 0 1)
    (:`1`
      (switch `int` (`KismetMathLibrary.RandomIntegerInRange` 0 1)
        (:`0`
          (`PrimitiveComponent.SetMaterial` (`self.Road`) 0 "/Engine/MapTemplates/Materials/BasicAsset01.BasicAsset01")
          (`|SpawnActorFromClass` "/Game/BP_Car.BP_Car_C" (`KismetMathLibrary.MakeTransform` (+ (`SceneComponent.K2_GetComponentLocation` _arrow2) (0.0 -50000.0 0.0)) (`SceneComponent.GetSocketRotation` _arrow2 "None")) "Undefined" "OverrideRootScale" null null))
        (:`1`
          (if (not (`self.Spawned`))
            (`PrimitiveComponent.SetMaterial` (`self.Road`) 0 "/Engine/MapTemplates/Materials/BasicAsset01.BasicAsset01")
            (`|SpawnActorFromClass` "/Game/BP_Car.BP_Car_C" (`KismetMathLibrary.MakeTransform` (+ (`SceneComponent.K2_GetComponentLocation` _arrow) (0.0 50000.0 0.0)) (`SceneComponent.GetSocketRotation` _arrow "None")) "Undefined" "OverrideRootScale" null null)
            (set `self.Spawned` true)
            (`KismetSystemLibrary.Delay` 7.0)
            (set `self.Spawned` false)))))))

(event `self.Box.OnComponentEndOverlap`
  (params (OverlappedComponent :type "PrimitiveComponent Object Reference") (OtherActor :type "Actor Object Reference") (OtherComp :type "PrimitiveComponent Object Reference") (OtherBodyIndex :type Integer))
  (cast `/Game/BP_Car` OtherActor)
  (`PrimitiveComponent.SetMaterial` (`self.Road`) 0 "/Engine/BasicShapes/BasicShapeMaterial.BasicShapeMaterial"))

(fn `UserConstructionScript`)